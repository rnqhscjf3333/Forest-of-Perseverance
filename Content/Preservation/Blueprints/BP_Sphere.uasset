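; BP_Sphere is a moving hazard actor that knocks the third-person character away on overlap.
; From BeginPlay, a timeline offsets it from its start position along GoArrow's forward vector, scaled by a travel distance.
; Each update also plays a second timeline that adds a vertical offset to the current location.
; On overlap, PowerArrow turns toward the player and supplies the direction for a Power-scaled velocity-change impulse.
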(event `self.ReceiveBeginPlay`
  (set `self.최초위치` (`self.K2_GetActorLocation`))
  (bind (_direction `_새_트랙_0`) (`Timeline|타임라인`)
    (:`Update`
      (`self.K2_SetActorLocation` (+ (`self.최초위치`) (* (`SceneComponent.GetForwardVector` (`self.GoArrow`)) `_새_트랙_0` (`self.이동거리`))))
      (bind (_direction_2 `_새_트랙_0_2`) (`Timeline|타임라인_0`)
        (:`Update`
          (`self.K2_SetActorRelativeLocation` (+ (* (`KismetMathLibrary.Vector_Up`) `_새_트랙_0_2` 10.0) (`self.K2_GetActorLocation`))))))))

(event `self.ReceiveActorBeginOverlap`
  (params (OtherActor :type "Actor Object Reference"))
  (`SceneComponent.K2_SetRelativeRotation` (`self.PowerArrow`) (`KismetMathLibrary.FindLookAtRotation` (`SceneComponent.K2_GetComponentLocation` (`self.PowerArrow`)) (`self.K2_GetActorLocation` (`GameplayStatics.GetPlayerCharacter` 0))) false false)
  (bind _asbp_third_person_character (cast `/Game/ThirdPerson/Blueprints/BP_ThirdPersonCharacter` OtherActor))
  (`CharacterMovementComponent.AddImpulse` (`Character.CharacterMovement` _asbp_third_person_character) (* (`SceneComponent.GetForwardVector` (`self.PowerArrow`)) (`self.Power`)) true))

(fn `NewFunction`
  (returns (StaticMeshComponent :type "StaticMeshComponent Object Reference"))
  (return (`self.StaticMeshComponent`)))

(fn `UserConstructionScript`)