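; BP_RedSpore is a moving hazard that knocks the player character back on contact.
; From BeginPlay, one timeline moves it along GoArrow over a set distance, while a second, started from that timeline's updates, adds vertical offsets.
; On overlap, PowerArrow turns toward the player and supplies a horizontal velocity-change impulse scaled by Power.
; A Hit widget appears only when the character's Hitcul counter has run out, which then resets.
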(event `self.ReceiveBeginPlay`
  (set `self.최초위치` (`self.K2_GetActorLocation`))
  (bind (_direction `_새_트랙_0`) (`Timeline|타임라인`)
    (:`Update`
      (`self.K2_SetActorLocation` (+ (`self.최초위치`) (* (`SceneComponent.GetForwardVector` (`self.GoArrow`)) `_새_트랙_0` (`self.이동거리`))))
      (bind (_direction_2 `_새_트랙_0_2`) (`Timeline|타임라인_0`)
        (:`Update`
          (`self.K2_SetActorRelativeLocation` (+ (* (`KismetMathLibrary.Vector_Up`) `_새_트랙_0_2` 10.0) (`self.K2_GetActorLocation`))))))))

(event `self.ReceiveActorBeginOverlap`
  (params (OtherActor :type "Actor Object Reference"))
  (bind (_returnvalue_x _returnvalue_y) (`KismetMathLibrary.BreakVector` (`SceneComponent.GetForwardVector` (`self.PowerArrow`))))
  (bind (_returnvalue_x_2 _returnvalue_y_2) (`KismetMathLibrary.BreakVector` (* (`KismetMathLibrary.Normal` (`KismetMathLibrary.MakeVector` _returnvalue_x _returnvalue_y)) (`self.Power`))))
  (`SceneComponent.K2_SetRelativeRotation` (`self.PowerArrow`) (`KismetMathLibrary.FindLookAtRotation` (`SceneComponent.K2_GetComponentLocation` (`self.PowerArrow`)) (`self.K2_GetActorLocation` (`GameplayStatics.GetPlayerCharacter` 0))) false false)
  (bind _asbp_third_person_character (cast `/Game/ThirdPerson/Blueprints/BP_ThirdPersonCharacter` OtherActor))
  (`CharacterMovementComponent.AddImpulse` (`Character.CharacterMovement` _asbp_third_person_character) (`KismetMathLibrary.MakeVector` _returnvalue_x_2 _returnvalue_y_2) true)
  (if (<= (`/Game/ThirdPerson/Blueprints/BP_ThirdPersonCharacter.Hitcul` _asbp_third_person_character) 0)
    (set `/Game/ThirdPerson/Blueprints/BP_ThirdPersonCharacter.Hitcul` 30 _asbp_third_person_character)
    (bind _returnvalue (`|CreateWidget` "/Game/Preservation/UI/Hit.Hit_C"))
    (`UserWidget.AddToViewport` _returnvalue 0)
    (`/Game/Preservation/UI/Hit.Hit_Event` _returnvalue)))

(fn `NewFunction`
  (returns (StaticMeshComponent :type "StaticMeshComponent Object Reference"))
  (return (`self.StaticMeshComponent`)))

(fn `UserConstructionScript`)